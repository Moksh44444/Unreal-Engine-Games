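; GM_Shooty is the game mode for a round-based Counter-Terrorist versus Terrorist shooter.
; It caches team spawn points on login and has player controllers spawn at a random one for their team.
; Alive and dead maps track each player's team, and a death that empties a team scores the round.
; It then announces the winner, clears both maps and respawns all spawned players after a delay.
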(event `self.K2_PostLogin`
  (params (NewPlayer :type "PlayerController Object Reference"))
  (`KismetArrayLibrary.Array_AddUnique` (`self.ConnectedPlayers`) NewPlayer)
  (bind _outactors (`GameplayStatics.GetAllActorsOfClass` "/Game/Blueprints/SpawnPoints/BP_CounterterriostSpawnpoint.BP_CounterterriostSpawnpoint_C"))
  (set `self.CounterTerrioristSpawnPoint` _outactors)
  (bind _outactors_2 (`GameplayStatics.GetAllActorsOfClass` "/Game/Blueprints/SpawnPoints/BP_TerrioristSpawnPoint.BP_TerrioristSpawnPoint_C"))
  (set `self.TerrioristSpawnPoint` _outactors_2))

(event `RequestSpawnPlayer`
  (params (PlayerController :type "/Game/Blueprints/PC_Shooty Object Reference") (Team :type "Actor Class Reference"))
  (`/Game/Blueprints/PC_Shooty.SpawnPlayer` PlayerController Team (`KismetMathLibrary.SelectTransform` (`self.GetTransform` (`KismetArrayLibrary.Array_Random` (`self.CounterTerrioristSpawnPoint`))) (`self.GetTransform` (`KismetArrayLibrary.Array_Random` (`self.TerrioristSpawnPoint`))) (== Team "/Game/Blueprints/Players/BP_Counterterrorist.BP_Counterterrorist_C"))))

(event `AddPlayersToAliveMap`
  (params (Player :type "/Game/Blueprints/Players/BP_PlayerBase Object Reference (by ref)"))
  (bind _playersdead (`self.PlayersDead`))
  (if (`.ReturnValue` (`BlueprintMapLibrary.Map_Find` _playersdead Player))
    (`BlueprintMapLibrary.Map_Remove` _playersdead Player))
  (bind _playercontroller (message `/Game/Blueprints/Interface/INT_PlayerController.GetPlayerControllerRef` (`Pawn.GetController` Player)))
  (`BlueprintMapLibrary.Map_Add` (`self.PlayersAlive`) Player (`/Game/Blueprints/PC_Shooty.Team` _playercontroller)))

(event `AddPlayersToDeadMap`
  (params (Player :type "/Game/Blueprints/Players/BP_PlayerBase Object Reference"))
  (bind _playersalive (`self.PlayersAlive`))
  (if (`.ReturnValue` (`BlueprintMapLibrary.Map_Find` _playersalive Player))
    (`BlueprintMapLibrary.Map_Remove` _playersalive Player))
  (bind _playercontroller (message `/Game/Blueprints/Interface/INT_PlayerController.GetPlayerControllerRef` (`Pawn.GetController` Player)))
  (`BlueprintMapLibrary.Map_Add` (`self.PlayersDead`) Player (`/Game/Blueprints/PC_Shooty.Team` _playercontroller))
  (bind (_counterterroristsalive _terroristsalive) (`self.m_CheckAmountOfLivingPlayers`))
  (if (or (== _counterterroristsalive 0) (== _terroristsalive 0))
    (`self.f_AddTeamScore`)
    (for _array_element (`self.PlayersSpawned`)
      (bind _playercontroller_2 (message `/Game/Blueprints/Interface/INT_PlayerController.GetPlayerControllerRef` (`Pawn.GetController` _array_element)))
      (bind _values (`BlueprintMapLibrary.Map_Values` (`self.PlayersAlive`)))
      (bind _output (`|GetArrayItem` _values))
      (`/Game/Blueprints/PC_Shooty.UpdateTeamWinAnnouncement` _playercontroller_2 _output (`KismetMathLibrary.SelectInt` (`self.CounterTerroristScore`) (`self.TerroristScore`) (== _output "/Game/Blueprints/Players/BP_Counterterrorist.BP_Counterterrorist_C")) (`self.RespawnTime`)))
    (`BlueprintMapLibrary.Map_Clear` (`self.PlayersAlive`))
    (`BlueprintMapLibrary.Map_Clear` (`self.PlayersDead`))
    (`KismetSystemLibrary.Delay` (`self.RespawnTime`))
    (for _array_element_2 (`self.PlayersSpawned`)
      (`/Game/Blueprints/Players/BP_PlayerBase.SRV_AddPlayersToAliveMap` _array_element_2 _array_element_2)
      (`/Game/Blueprints/Players/BP_PlayerBase.Respawn` _array_element_2))))

(event `AddToPlayersSpawnedArray`
  (params (Player :type "/Game/Blueprints/Players/BP_PlayerBase Object Reference"))
  (bind _playersspawned (`self.PlayersSpawned`))
  (`KismetArrayLibrary.Array_Set` _playersspawned (`KismetArrayLibrary.Array_Length` _playersspawned) Player true))

(fn `f_AddTeamScore`
  (if (== (`self.CounterTerroristsAlive`) 0)
    (`/Engine/EditorBlueprintResources/StandardMacros.IncrementInt` (`self.TerroristScore`))
    (else
      (`/Engine/EditorBlueprintResources/StandardMacros.IncrementInt` (`self.CounterTerroristScore`)))))

(fn `GetGameModeRef`
  (returns (GameMode :type "/Game/Blueprints/GM_Shooty Object Reference"))
  (return self))

(fn `UserConstructionScript`)